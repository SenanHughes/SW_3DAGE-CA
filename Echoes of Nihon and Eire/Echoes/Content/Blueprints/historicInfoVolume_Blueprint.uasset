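; Trigger volume that shows historic item information when the third-person player character enters it.
; It creates a HistoricItemInfo widget at BeginPlay and keeps it for reuse.
; On overlap by BP_ThirdPersonCharacter it calls the character's MoveCamera and adds the widget to the viewport; on exit it calls ReturnCamera and removes the widget.
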(event `self.ReceiveBeginPlay`
  (bind _returnvalue (`|CreateWidget` "/Game/Widgets/historicItemInfo_Widget.historicItemInfo_Widget_C"))
  (set `self.historicInfoWidget` _returnvalue))

(event `self.ReceiveActorBeginOverlap`
  (params (OtherActor :type "Actor Object Reference"))
  (bind _asbp_third_person_character (cast `/Game/ThirdPerson/Blueprints/BP_ThirdPersonCharacter` OtherActor))
  (`/Game/ThirdPerson/Blueprints/BP_ThirdPersonCharacter.moveCamera` _asbp_third_person_character)
  (`UserWidget.AddToViewport` (`self.historicInfoWidget`) 0))

(event `self.ReceiveActorEndOverlap`
  (params (OtherActor :type "Actor Object Reference"))
  (bind _asbp_third_person_character (cast `/Game/ThirdPerson/Blueprints/BP_ThirdPersonCharacter` OtherActor))
  (`/Game/ThirdPerson/Blueprints/BP_ThirdPersonCharacter.returnCamera` _asbp_third_person_character)
  (`Widget.RemoveFromParent` (`self.historicInfoWidget`)))

(fn `UserConstructionScript`)