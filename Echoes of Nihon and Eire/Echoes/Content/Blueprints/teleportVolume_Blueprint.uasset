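; A teleport volume that lets the third-person character travel to the JapaneseShrine level by pressing E while inside it.
; Overlap begin and end add or remove an interact prompt widget, created at BeginPlay, and toggle a ready flag.
; Input is enabled on the actor from BeginPlay, so the E handler checks that flag, spawns a particle effect at the character, then opens the level after a short delay.
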(event `self.ReceiveBeginPlay`
  (`self.EnableInput` (`GameplayStatics.GetPlayerController` 0))
  (bind _returnvalue (`|CreateWidget` "/Game/Widgets/playerInteract_Widget.playerInteract_Widget_C"))
  (set `self.playerInteract` _returnvalue))

(event `self.ReceiveActorBeginOverlap`
  (params (OtherActor :type "Actor Object Reference"))
  (cast `/Game/ThirdPerson/Blueprints/BP_ThirdPersonCharacter` OtherActor)
  (`UserWidget.AddToViewport` (`self.playerInteract`) 0)
  (set `self.triggerReady` true))

(event `self.ReceiveActorEndOverlap`
  (params (OtherActor :type "Actor Object Reference"))
  (cast `/Game/ThirdPerson/Blueprints/BP_ThirdPersonCharacter` OtherActor)
  (`Widget.RemoveFromParent` (`self.playerInteract`))
  (set `self.triggerReady` false))

(event `Key|E`
  (params (Key :type "Key Structure"))
  (:`Pressed`
    (bind _asbp_third_person_character (cast `/Game/ThirdPerson/Blueprints/BP_ThirdPersonCharacter` (`GameplayStatics.GetPlayerCharacter` 0)))
    (if (`self.triggerReady`)
      (`GameplayStatics.SpawnEmitterAtLocation` "/Engine/Tutorial/SubEditors/TutorialAssets/TutorialParticleSystem.TutorialParticleSystem" (`self.K2_GetActorLocation` _asbp_third_person_character) (struct) (1.0 1.0 1.0) false)
      (`KismetSystemLibrary.Delay` 2.0)
      (`GameplayStatics.OpenLevelBySoftObjectPtr` "/Game/Levels/japaneseShrine_Level.japaneseShrine_Level"))))

(fn `UserConstructionScript`)